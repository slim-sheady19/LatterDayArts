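; VR character Blueprint that lets the player grab and release objects with the left and right grip inputs.
; On press, each hand's motion controller grips every component overlapping its collision sphere that implements VRGripInterface, using a relative offset.
; Only the last gripped component is stored per hand, and releasing the input drops just that one.
; Grip presses also print debug strings, and the construction script is empty.
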(event EventBeginPlay)

(event Collision|EventActorBeginOverlap
  (params (OtherActor :type Actor%20Object%20Reference)))

(event EventTick
  (params (DeltaSeconds :type Float%20%28single-precision%29)))

(event Input|ActionEvents|InputActionPrimaryGripRight
  (params (Key :type Key%20Structure :default "None"))
  (:Pressed
    (Development|PrintString "rightgrip")
    (for _array_element (Class|PrimitiveComponent|GetOverlappingComponents (Variables|Default|GetRSphereColliision))
      (if (Utilities|DoesObjectImplementInterface _array_element "/Script/VRExpansionPlugin.VRGripInterface")
        (Class|GripMotionControllerComponent|GripObjectbyInterface (Variables|Default|GetRightMotionController) _array_element (Math|Transform|MakeTransform "0, 0, 0" "0, 0, 0" "1,1,1") true "None" "None" false)
        (if true
          (Variables|Default|SetGrabRight _array_element)))))
  (:Released
    (Class|GripMotionControllerComponent|DropObjectbyInterface (Variables|Default|GetRightMotionController) (Variables|Default|GetGrabRight) 0 "0, 0, 0" "0, 0, 0")))

(event Input|ActionEvents|InputActionPrimaryGripLeft
  (params (Key :type Key%20Structure :default "None"))
  (:Pressed
    (Development|PrintString "LEFTGRIP")
    (for _array_element (Class|PrimitiveComponent|GetOverlappingComponents (Variables|Default|GetLSphereCollision))
      (if (Utilities|DoesObjectImplementInterface _array_element "/Script/VRExpansionPlugin.VRGripInterface")
        (Class|GripMotionControllerComponent|GripObjectbyInterface (Variables|Default|GetLeftMotionController) _array_element (Math|Transform|MakeTransform "0, 0, 0" "0, 0, 0" "1,1,1") true "None" "None" false)
        (if true
          (Variables|Default|SetGrabLeft _array_element)))))
  (:Released
    (Class|GripMotionControllerComponent|DropObjectbyInterface (Variables|Default|GetLeftMotionController) (Variables|Default|GetGrabLeft) 0 "0, 0, 0" "0, 0, 0")))

(fn ConstructionScript)